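; BP_Windmill is a windmill actor whose fan spins continuously.
; BeginPlay stores the fan component's relative location and rotation.
; Each Tick adds a fixed pitch step to the stored rotation and applies it at the stored location, without delta-time scaling, so spin speed depends on frame rate.
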(event EventBeginPlay
  (bind _windmill_fan (Variables|Default|GetWindMill_Fan))
  (bind _returnvalue (Transformation|GetRelativeTransform _windmill_fan))
  (Variables|Default|SetLocationOfFan (.location _returnvalue))
  (Variables|Default|SetRotationOfFan (.rotation _returnvalue)))

(event Collision|EventActorBeginOverlap
  (params (OtherActor :type Actor%20Object%20Reference)))

(event EventTick
  (params (DeltaSeconds :type Float%20%28single-precision%29))
  (Transformation|SetRelativeLocationAndRotation (Variables|Default|GetWindMill_Fan) (Variables|Default|GetLocationOfFan) (Math|Rotator|MakeRotator (.roll (Variables|Default|GetRotationOfFan)) (+ (.pitch (Variables|Default|GetRotationOfFan)) 0.8) (.yaw (Variables|Default|GetRotationOfFan))) false false)
  (Variables|Default|SetRotationOfFan (Math|Rotator|MakeRotator (.roll (Variables|Default|GetRotationOfFan)) (+ (.pitch (Variables|Default|GetRotationOfFan)) 0.8) (.yaw (Variables|Default|GetRotationOfFan)))))

(fn ConstructionScript)